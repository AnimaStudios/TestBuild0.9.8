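; Inventory game mode that persists world pickups and containers in an SG_GameWorld save slot named after the level.
; On first load it records placed BP_Pickup and BP_Container actors; later loads destroy them and respawn from saved data.
; Parallel actor and info arrays share indices for save updates.
; Container adds use data table stack limits, spilling overflow into other slots or throwing it via the interacting player.
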(event `self.ReceiveBeginPlay`
  (bind _savegameworld (`self.SaveGameWorld`))
  (bind _returnvalue (`GameplayStatics.GetCurrentLevelName` true))
  (bind _savegameworld_2 (`self.Initalize_GameWorldSave` _returnvalue))
  (`/Engine/EditorBlueprintResources/StandardMacros.IsValid` _savegameworld_2
    (:`Is Valid`
      (bind _isfirsttimeloadingmap (`/Game/Inventory/SavedData/SG_GameWorld.IsFirstTimeLoadingMap` _savegameworld_2))
      (if _isfirsttimeloadingmap
        _
        (else
          _))
      (`self.Setup_PickupActors` (`/Game/Inventory/SavedData/SG_GameWorld.All_PickupActorsInfo` _savegameworld_2) _isfirsttimeloadingmap)
      (`self.Setup_ContainerActors` (`/Game/Inventory/SavedData/SG_GameWorld.All_containerActorInfo` _savegameworld_2) _isfirsttimeloadingmap)
      (if _isfirsttimeloadingmap
        (set `/Game/Inventory/SavedData/SG_GameWorld.IsFirstTimeLoadingMap` false _savegameworld)
        (`GameplayStatics.SaveGameToSlot` _savegameworld (`self.GameWorldSaveSlot`))
        (for _array_element (`self.All_SavedContainersActors`)
          (`/Game/Inventory/BP_Container.RefreshContents` _array_element self))))))

(fn `Add Saved Pickup Actor`
  (params (BP_Pickup :type "/Game/Inventory/BP_Pickup Object Reference"))
  (`KismetArrayLibrary.Array_AddUnique` (`self.All_SavedPickupActors`) BP_Pickup))

(fn `Add_ItemToContainer`
  (params (Contents :type "Array of /Game/Inventory/S_InventoryContents Structure") (BP_Container :type "/Game/Inventory/BP_Container Object Reference") (InventoryIndex :type Integer))
  (locals (Lol_ContainerWorldIndex :type Integer :default 0) (Lol_InventoryIndex :type Integer :default 0) (Lol_ContainerInventoryContents :type "/Game/Inventory/S_InventoryContents Structure") (Lcl_ContentsToAdd :type "/Game/Inventory/S_InventoryContents Structure") (Lol_IsSlotFound :type Boolean) (Lcl_CanStackItem :type Boolean) (Lcl_IsStackLimited :type Boolean) (Lcl_MaxStackSize :type Integer) (Lcl_AllItemsAdded :type Boolean) (Lcl_NewStackSize :type Integer) (Lcl_AmountLeftToAdd :type Integer))
  (bind _lol_containerworldindex (`local.Lol_ContainerWorldIndex`))
  (bind (_itemrowname _itemamount) (break `/Game/Inventory/S_InventoryContents` (`local.Lcl_ContentsToAdd`)))
  (bind (_itemrowname_2 _itemamount_2) (break `/Game/Inventory/S_InventoryContents` (`local.Lol_ContainerInventoryContents`)))
  (bind _output_get (set `local.Lol_ContainerWorldIndex` (`KismetArrayLibrary.Array_Find` (`self.All_SavedContainersActors`) BP_Container)))
  (if (>= _output_get 0)
    (bind _output_get_2 (set `local.Lcl_ContentsToAdd` (`|GetArrayItem` (`local.Contents`))))
    (set `local.Lol_InventoryIndex` InventoryIndex)
    (set `local.Lol_ContainerInventoryContents` (`|GetArrayItem` (`/Game/Inventory/BP_Container.ContainerContents` (`local.BP_Container`)) (`local.Lol_InventoryIndex`)))
    (bind _returnvalue (`|GetDataTableRow` "/Game/Inventory/TB_PickUpItemInfo.TB_PickUpItemInfo" (`.ItemRowNAme_3_03A6F83347ECA63487A0DAA65D30ACFB` (break `/Game/Inventory/S_InventoryContents` _output_get_2)))
      (:`then`
        (bind (_pickupname _pickupmesh _pickupmesh_scale _showpickupname _pickupmeshoffset _hud_icon _maxstacksize) (break `/Game/Inventory/S_PickUpItemInfo` _returnvalue))
        (switch `int` _maxstacksize
          (:`Default`
            (set `local.Lcl_CanStackItem` true)
            (set `local.Lcl_IsStackLimited` true)
            (set `local.Lcl_MaxStackSize` _maxstacksize))
          (:`-1`
            (set `local.Lcl_CanStackItem` false)
            (set `local.Lcl_IsStackLimited` true)
            (set `local.Lcl_MaxStackSize` 1))
          (:`0`
            (set `local.Lcl_CanStackItem` true)
            (set `local.Lcl_IsStackLimited` false)))
        (set `local.Lcl_AllItemsAdded` true :!label _label)
        (set `local.Lcl_NewStackSize` 0)
        (set `local.Lcl_AmountLeftToAdd` 0)
        (set `local.Lol_IsSlotFound` false)
        (if (< (`local.Lol_InventoryIndex`) 0)
          (for (_array_element _array_index) (`/Game/Inventory/BP_Container.ContainerContents` (`local.BP_Container`)) :!label _label_2
            (if (== (`.ItemRowNAme_3_03A6F83347ECA63487A0DAA65D30ACFB` (break `/Game/Inventory/S_InventoryContents` _array_element)) "Empty")
              (set `local.Lol_IsSlotFound` true)
              (set `local.Lol_InventoryIndex` _array_index)
              (break)))
          (if (`local.Lol_IsSlotFound`)
            (set `local.Lcl_NewStackSize` (`.ItemAmount_6_5F407C944CCD8EFBF9780CB5F8F7A858` (break `/Game/Inventory/S_InventoryContents` (`local.Lcl_ContentsToAdd`))) :!label _label_3)
            (if (`local.Lcl_IsStackLimited`)
              (if (not (<= (`local.Lcl_NewStackSize`) (`local.Lcl_MaxStackSize`)))
                (set `local.Lcl_AmountLeftToAdd` (- (`local.Lcl_NewStackSize`) (`local.Lcl_MaxStackSize`)))
                (set `local.Lcl_NewStackSize` (`local.Lcl_MaxStackSize`))
                (set `local.Lcl_AllItemsAdded` false)))
            (`KismetArrayLibrary.Array_Set` (`/Game/Inventory/BP_Container.ContainerContents` (`local.BP_Container`)) (`local.Lol_InventoryIndex`) (make `/Game/Inventory/S_InventoryContents` (`.ItemRowNAme_3_03A6F83347ECA63487A0DAA65D30ACFB` (break `/Game/Inventory/S_InventoryContents` (`local.Lcl_ContentsToAdd`))) (`local.Lcl_NewStackSize`)) true)
            (if (`local.Lcl_AllItemsAdded`) :!label _label_4
              _
              (else
                (setmembers `/Game/Inventory/S_InventoryContents` :`StructRef` (`local.Lcl_ContentsToAdd`) :`ItemAmount` (`local.Lcl_AmountLeftToAdd`))
                (set `local.Lol_InventoryIndex` -1)
                (goto _label)))
            (else
              (if (`local.Lcl_CanStackItem`)
                (for (_array_element_2 _array_index_2) (`/Game/Inventory/BP_Container.ContainerContents` (`local.BP_Container`))
                  (bind (_itemrowname_3 _itemamount_3) (break `/Game/Inventory/S_InventoryContents` _array_element_2))
                  (if (== _itemrowname_3 (`.ItemRowNAme_3_03A6F83347ECA63487A0DAA65D30ACFB` (break `/Game/Inventory/S_InventoryContents` (`local.Lcl_ContentsToAdd`))))
                    (if (or (and (`local.Lcl_CanStackItem`) (not (`local.Lcl_IsStackLimited`))) (and (`local.Lcl_CanStackItem`) (`local.Lcl_IsStackLimited`) (< _itemamount_3 (`local.Lcl_MaxStackSize`))))
                      (set `local.Lol_IsSlotFound` true)
                      (set `local.Lol_InventoryIndex` _array_index_2)
                      (set `local.Lol_ContainerInventoryContents` _array_element_2)
                      (break))))
                (if (`local.Lol_IsSlotFound`)
                  (set `local.Lcl_NewStackSize` (+ _itemamount_2 (`.ItemAmount_6_5F407C944CCD8EFBF9780CB5F8F7A858` (break `/Game/Inventory/S_InventoryContents` (`local.Lcl_ContentsToAdd`)))) :!label _label_5)
                  (if (`local.Lcl_IsStackLimited`)
                    (if (not (<= (`local.Lcl_NewStackSize`) (`local.Lcl_MaxStackSize`)))
                      (set `local.Lcl_AmountLeftToAdd` (- (`local.Lcl_NewStackSize`) (`local.Lcl_MaxStackSize`)))
                      (set `local.Lcl_NewStackSize` (`local.Lcl_MaxStackSize`))
                      (set `local.Lcl_AllItemsAdded` false)))
                  (`KismetArrayLibrary.Array_Set` (`/Game/Inventory/BP_Container.ContainerContents` (`local.BP_Container`)) (`local.Lol_InventoryIndex`) (make `/Game/Inventory/S_InventoryContents` _itemrowname_2 (`local.Lcl_NewStackSize`)) true)
                  (goto _label_4)
                  (else
                    (`KismetSystemLibrary.PrintString` "inventroy full cannot add item" true true (struct :`R` 1.0 :`B` 0.083431 :`A` 1.0) 15.0)))
                (else
                  (`KismetSystemLibrary.PrintString` "Inventory full! Item cannot stack!" true true (struct :`R` 1.0 :`G` 0.203125 :`B` 0.221132 :`A` 1.0) 5.0)))
              (`/Game/Inventory/BP_InvComp_Character.ThrowItem` (`|GetArrayItem` (`/Game/Inventory/BP_Container.InteractingPlayers` (`local.BP_Container`))) _itemrowname (`|MakeArray` (make `/Game/Inventory/S_InventoryContents` _itemrowname _itemamount)) true)))
          (elif (== (`.ItemRowNAme_3_03A6F83347ECA63487A0DAA65D30ACFB` (break `/Game/Inventory/S_InventoryContents` (`local.Lol_ContainerInventoryContents`))) (`.ItemRowNAme_3_03A6F83347ECA63487A0DAA65D30ACFB` (break `/Game/Inventory/S_InventoryContents` (`local.Lcl_ContentsToAdd`))))
            (if (`local.Lcl_CanStackItem`)
              (goto _label_5)
              (else
                (goto _label_2)))
            (elif (== (`.ItemRowNAme_3_03A6F83347ECA63487A0DAA65D30ACFB` (break `/Game/Inventory/S_InventoryContents` (`local.Lol_ContainerInventoryContents`))) "Empty")
              (goto _label_3)
              (else
                (goto _label_2)))))
        (`KismetArrayLibrary.Array_Set` (`self.All_SavedContainersActors`) _lol_containerworldindex BP_Container true)
        (`KismetArrayLibrary.Array_Set` (`self.All_SavedContainersActors_Info`) _lol_containerworldindex (make `/Game/Inventory/SavedData/WorldInfoContainers` (`/Game/Inventory/BP_Container.ContainerRowName` BP_Container) (`/Game/Inventory/BP_Container.ContainerContents` BP_Container) (`Actor.GetTransform` BP_Container)) true)
        (`self.UpdateSaveContainerActors` (`self.All_SavedContainersActors_Info`))
        (`/Game/Inventory/BP_Container.ContainerContentsChanged` BP_Container)
        (return)))))

(fn `Initalize_GameWorldSave`
  (params (SaveSlotName :type String))
  (returns (SaveGameWorld :type "/Game/Inventory/SavedData/SG_GameWorld Object Reference"))
  (bind _output_get (set `self.GameWorldSaveSlot` SaveSlotName))
  (bind _returnvalue (`GameplayStatics.DoesSaveGameExist` _output_get))
  (if _returnvalue
    (bind _returnvalue_2 (`GameplayStatics.LoadGameFromSlot` (`self.GameWorldSaveSlot`)))
    (bind _assg_game_world (cast `/Game/Inventory/SavedData/SG_GameWorld` _returnvalue_2))
    (set `self.SaveGameWorld` _assg_game_world)
    (else
      (bind _returnvalue_3 (`GameplayStatics.CreateSaveGameObject` "/Game/Inventory/SavedData/SG_GameWorld.SG_GameWorld_C"))
      (bind _output_get_2 (set `self.SaveGameWorld` _returnvalue_3))
      (`GameplayStatics.SaveGameToSlot` _output_get_2 (`self.GameWorldSaveSlot`))))
  (return (`self.SaveGameWorld`)))

(fn `Remove_ItemFromContainer`
  (params (Contents :type "Array of /Game/Inventory/S_InventoryContents Structure") (BP_Container :type "/Game/Inventory/BP_Container Object Reference") (InventroyIndex :type Integer))
  (locals (Lcl_ContainerWorldIndex :type Integer :default 0) (Lcl_NewAmount :type Integer))
  (bind _lcl_containerworldindex (`local.Lcl_ContainerWorldIndex`))
  (bind (_itemrowname _itemamount) (break `/Game/Inventory/S_InventoryContents` (`|GetArrayItem` (`/Game/Inventory/BP_Container.ContainerContents` BP_Container) InventroyIndex)))
  (bind _output_get (set `local.Lcl_ContainerWorldIndex` (`KismetArrayLibrary.Array_Find` (`self.All_SavedContainersActors`) BP_Container)))
  (if (>= _output_get 0)
    (bind _output_get_2 (set `local.Lcl_NewAmount` (- _itemamount (`.ItemAmount_6_5F407C944CCD8EFBF9780CB5F8F7A858` (break `/Game/Inventory/S_InventoryContents` (`|GetArrayItem` Contents))))))
    (if (<= _output_get_2 0)
      (`KismetArrayLibrary.Array_Set` (`/Game/Inventory/BP_Container.ContainerContents` (`local.BP_Container`)) 0 (make `/Game/Inventory/S_InventoryContents` "Empty"))
      (else
        (`KismetArrayLibrary.Array_Set` (`/Game/Inventory/BP_Container.ContainerContents` (`local.BP_Container`)) InventroyIndex (make `/Game/Inventory/S_InventoryContents` _itemrowname (`local.Lcl_NewAmount`)))))
    (`KismetArrayLibrary.Array_Set` (`/Game/Inventory/BP_Container.ContainerContents` (`local.BP_Container`)) InventroyIndex (make `/Game/Inventory/S_InventoryContents` "Empty"))
    (`KismetArrayLibrary.Array_Set` (`self.All_SavedContainersActors`) _lcl_containerworldindex BP_Container true)
    (`KismetArrayLibrary.Array_Set` (`self.All_SavedContainersActors_Info`) _lcl_containerworldindex (make `/Game/Inventory/SavedData/WorldInfoContainers` (`/Game/Inventory/BP_Container.ContainerRowName` BP_Container) (`/Game/Inventory/BP_Container.ContainerContents` BP_Container) (`Actor.GetTransform` BP_Container)) true)
    (`self.UpdateSaveContainerActors` (`self.All_SavedContainersActors_Info`))
    (`/Game/Inventory/BP_Container.ContainerContentsChanged` BP_Container)
    (return)))

(fn `Remove_SavedPickupActor`
  (params (BP_Pickup :type "/Game/Inventory/BP_Pickup Object Reference"))
  (locals (Lol_IndexToRemove :type Integer :default 0))
  (bind _lol_indextoremove (`local.Lol_IndexToRemove`))
  (bind _output_get (set `local.Lol_IndexToRemove` (`KismetArrayLibrary.Array_Find` (`self.All_SavedPickupActors`) BP_Pickup)))
  (if (>= _output_get 0)
    (`KismetSystemLibrary.PrintString` "Pickup Remove From Savegame " true true (struct :`R` 0.131702 :`G` 1.0 :`A` 1.0))
    (`KismetArrayLibrary.Array_Remove` (`self.All_SAvedPickupActorsInfo`) _lol_indextoremove)
    (`KismetArrayLibrary.Array_Remove` (`self.All_SavedPickupActors`) _lol_indextoremove)
    (`self.Update_SavedPickupActors` (`self.All_SAvedPickupActorsInfo`))
    (else
      (`KismetSystemLibrary.PrintString` "Pickup Remove From Savegame failed" true true (struct :`R` 1.0 :`G` 0.009794 :`A` 1.0))))
  (return))

(fn `SaveContainerContents`
  (params (BP_Container :type "/Game/Inventory/BP_Container Object Reference"))
  (locals (Lcl_ContainerWorldIndex :type Integer :default 0))
  (bind _lcl_containerworldindex (`local.Lcl_ContainerWorldIndex`))
  (bind _output_get (set `local.Lcl_ContainerWorldIndex` (`KismetArrayLibrary.Array_Find` (`self.All_SavedContainersActors`) BP_Container)))
  (if (>= _output_get 0)
    (`KismetArrayLibrary.Array_Set` (`self.All_SavedContainersActors`) _lcl_containerworldindex BP_Container true)
    (`KismetArrayLibrary.Array_Set` (`self.All_SavedContainersActors_Info`) _lcl_containerworldindex (make `/Game/Inventory/SavedData/WorldInfoContainers` (`/Game/Inventory/BP_Container.ContainerRowName` BP_Container) (`/Game/Inventory/BP_Container.ContainerContents` BP_Container) (`Actor.GetTransform` BP_Container)) true)
    (`self.UpdateSaveContainerActors` (`self.All_SavedContainersActors_Info`))))

(fn `Setup_ContainerActors`
  (params (All_ContainersActorInfo :type "Array of /Game/Inventory/SavedData/WorldInfoContainers Structure") (IsFirstTimeLoadingMap :type Boolean))
  (if IsFirstTimeLoadingMap
    (`KismetSystemLibrary.PrintString` "No Saved Container data, SAving world info to savegame" true true (struct :`R` 1.0 :`G` 0.013739 :`A` 1.0))
    (bind _outactors (`GameplayStatics.GetAllActorsOfClass` "/Game/Inventory/BP_Container.BP_Container_C"))
    (bind _output_get (set `self.All_SavedContainersActors` _outactors))
    (for (_array_element _array_index) _output_get
      (`KismetArrayLibrary.Array_Set` (`self.All_SavedContainersActors_Info`) _array_index (make `/Game/Inventory/SavedData/WorldInfoContainers` (`/Game/Inventory/BP_Container.ContainerRowName` _array_element) (`/Game/Inventory/BP_Container.ContainerContents` _array_element) (`Actor.GetTransform` _array_element)) true))
    (`self.UpdateSaveContainerActors` (`self.All_SavedContainersActors_Info`))
    (else
      (`KismetSystemLibrary.PrintString` "Saved Container data found, loading world contents" true true (struct :`R` 0.361903 :`G` 1.0 :`A` 1.0))
      (bind _outactors_2 (`GameplayStatics.GetAllActorsOfClass` "/Game/Inventory/BP_Container.BP_Container_C"))
      (for _array_element_2 _outactors_2
        (`Actor.K2_DestroyActor` _array_element_2))
      (for _array_element_3 All_ContainersActorInfo
        (bind (_containerrowname _containercontents _worldtransform) (break `/Game/Inventory/SavedData/WorldInfoContainers` _array_element_3))
        (bind _returnvalue (`|SpawnActorFromClass` :`Class` "/Game/Inventory/BP_Container.BP_Container_C" :`SpawnTransform` _worldtransform :`CollisionHandlingOverride` "Undefined" :`TransformScaleMethod` "OverrideRootScale" :`ContainerContents` _containercontents :`ContainerRowName` _containerrowname :`Instigator` null))
        (`/Engine/EditorBlueprintResources/StandardMacros.IsValid` _returnvalue
          (:`Is Valid`
            (bind _returnvalue_2 (`KismetArrayLibrary.Array_Add` (`self.All_SavedContainersActors`) _returnvalue))
            (`KismetArrayLibrary.Array_Set` (`self.All_SavedContainersActors_Info`) _returnvalue_2 _array_element_3 true))))))
  (return))

(fn `Setup_PickupActors`
  (params (AllPickupActorsInfo :type "Array of /Game/Inventory/SavedData/S_WorldInfo_PickupItem Structure") (IsFirstTimeLoadingMap :type Boolean))
  (if IsFirstTimeLoadingMap
    (`KismetSystemLibrary.PrintString` "No saved pickup data, saving world info to save game" true true (struct :`R` 1.0 :`G` 0.048107 :`A` 1.0))
    (bind _outactors (`GameplayStatics.GetAllActorsOfClass` "/Game/Inventory/BP_Pickup.BP_Pickup_C"))
    (bind _output_get (set `self.All_SavedPickupActors` _outactors))
    (for (_array_element _array_index) _output_get
      (`KismetArrayLibrary.Array_Set` (`self.All_SavedPickupActorsInfo`) _array_index (make `/Game/Inventory/SavedData/S_WorldInfo_PickupItem` (`/Game/Inventory/BP_Pickup.ItemRowName` _array_element) (`/Game/Inventory/BP_Pickup.ItemContents` _array_element) (`Actor.GetTransform` _array_element)) true))
    (`self.Update_SavedPickupActors` (`self.All_SavedPickupActorsInfo`))
    (else
      (`KismetSystemLibrary.PrintString` "Saved pickup data found loading world contents" true true (struct :`R` 0.0201 :`G` 1.0 :`A` 1.0))
      (bind _outactors_2 (`GameplayStatics.GetAllActorsOfClass` "/Game/Inventory/BP_Pickup.BP_Pickup_C"))
      (for _array_element_2 _outactors_2
        (`Actor.K2_DestroyActor` _array_element_2))
      (for _array_element_3 (`local.AllPickupActorsInfo`)
        (bind (_itemrowname _itemcontents _worldtransform) (break `/Game/Inventory/SavedData/S_WorldInfo_PickupItem` _array_element_3))
        (bind _returnvalue (`|SpawnActorFromClass` "/Game/Inventory/BP_Pickup.BP_Pickup_C" _worldtransform "Undefined" "OverrideRootScale" null _itemrowname _itemcontents null))
        (`/Engine/EditorBlueprintResources/StandardMacros.IsValid` _returnvalue
          (:`Is Valid`
            (bind _returnvalue_2 (`KismetArrayLibrary.Array_Add` (`self.All_SavedPickupActors`) _returnvalue))
            (`KismetArrayLibrary.Array_Set` (`self.All_SavedPickupActorsInfo`) _returnvalue_2 _array_element_3 true))))))
  (return))

(fn `SpawnDynamicLoot`
  ;[0 0 0] Spawns loot and a chest in the map
  (`|SpawnActorFromClass` "/Game/Inventory/BP_Pickup.BP_Pickup_C" (`KismetMathLibrary.MakeTransform` (1750.0 1900.0 200.0)) "Undefined" "OverrideRootScale" null "Orb" (`|MakeArray` (make `/Game/Inventory/S_InventoryContents` "Orb" 1)) null)
  (`|SpawnActorFromClass` "/Game/Inventory/BP_Pickup.BP_Pickup_C" (`KismetMathLibrary.MakeTransform` (1750.0 2100.0 200.0)) "Undefined" "OverrideRootScale" null "Orb" (`|MakeArray` (make `/Game/Inventory/S_InventoryContents` "Orb" 1)) null)
  (`|SpawnActorFromClass` :`Class` "/Game/Inventory/BP_Container.BP_Container_C" :`SpawnTransform` (`KismetMathLibrary.MakeTransform` (1300.0 1900.0 200.0)) :`CollisionHandlingOverride` "Undefined" :`TransformScaleMethod` "OverrideRootScale" :`ContainerContents` (`|MakeArray` (make `/Game/Inventory/S_InventoryContents` "Fan" 2) (make `/Game/Inventory/S_InventoryContents` "dish" 2)) :`ContainerRowName` "Crate_Big" :`Instigator` null))

(fn `Update_SavedPickupActors`
  (params (AllPickupActorsInfo :type "Array of /Game/Inventory/SavedData/S_WorldInfo_PickupItem Structure"))
  (bind _savegameworld (`self.SaveGameWorld`))
  (set `/Game/Inventory/SavedData/SG_GameWorld.All_PickupActorsInfo` AllPickupActorsInfo _savegameworld)
  (`GameplayStatics.SaveGameToSlot` _savegameworld (`self.GameWorldSaveSlot`))
  (return))

(fn `UpdateSaveContainerActors`
  (params (All_ContainerActorsInfo :type "Array of /Game/Inventory/SavedData/WorldInfoContainers Structure"))
  (bind _savegameworld (`self.SaveGameWorld`))
  (set `/Game/Inventory/SavedData/SG_GameWorld.All_containerActorInfo` All_ContainerActorsInfo _savegameworld)
  (`GameplayStatics.SaveGameToSlot` _savegameworld (`self.GameWorldSaveSlot`)))