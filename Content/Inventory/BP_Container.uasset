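; BP_Container is an interactable world inventory container with mesh, scale and slot count set server-side from a data table row.
; The server pads slots with "Empty" entries on BeginPlay; interaction registers the player and opens the container.
; Content changes update each registered player's grid, and clearing also saves through the game mode component.
; RefreshContents waits for readiness, then empties every slot; its re-add call to the game mode is disconnected.
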(event `RefreshContents`
  (params (Gamemode :type "/Game/Inventory/BP_InvCompGamemode Object Reference"))
  (if (`self.IsContainerReady`) :!label _label
    (set `self.Temp_RefreshContents` (`self.ContainerContents`))
    (for (_ _array_index) (`self.ContainerContents`)
      (`KismetArrayLibrary.Array_Set` (`self.ContainerContents`) _array_index (make `/Game/Inventory/S_InventoryContents` "Empty")))
    (for (_array_element _array_index_2) (`self.Temp_RefreshContents`)
      _)
    (else
      (`KismetSystemLibrary.DelayUntilNextTick`)
      (goto _label))))

(event `self.ReceiveBeginPlay`
  (if (`KismetSystemLibrary.IsServer`)
    (for _index (range (`KismetArrayLibrary.Array_Length` (`self.ContainerContents`)) (`self.InventorySize`))
      (`KismetArrayLibrary.Array_Set` (`self.ContainerContents`) _index (make `/Game/Inventory/S_InventoryContents` "Empty") true))
    (set `self.IsContainerReady` true)))

(event `/Game/Inventory/BPI_InteractableActor.InteractWithActor`
  (params (PlayerCharacter :type "/Game/Inventory/BP_InvComp_Character Object Reference"))
  (`KismetArrayLibrary.Array_AddUnique` (`self.InteractingPlayers`) PlayerCharacter)
  (set `/Game/Inventory/BP_InvComp_Character.OpenedContainer` self PlayerCharacter)
  (`/Game/Inventory/BP_InvComp_Character.OpenContainer` PlayerCharacter self))

(event `ContainerContentsChanged`
  (for _array_element (`self.InteractingPlayers`)
    (`/Game/Inventory/BP_InvComp_Controller.HUD_UpdateInventoryGrid` (`/Game/Inventory/BP_InvComp_Character.BP_InvComponent_Controller` _array_element) (`self.ContainerContents`) false true)))

(event `ClearInventoryContents`
  (for (_ _array_index) (`self.ContainerContents`)
    (`KismetArrayLibrary.Array_Set` (`self.ContainerContents`) _array_index (make `/Game/Inventory/S_InventoryContents` "Empty")))
  (`self.ContainerContentsChanged`)
  (`/Game/Inventory/BP_InvCompGamemode.SaveContainerContents` (`self.GetComponentByClass` (`GameplayStatics.GetGameMode`) "/Game/Inventory/BP_InvCompGamemode.BP_InvCompGamemode_C") self))

(fn `Get_InteractHintText`
  (returns (HintText :type Text))
  (return "Open container"))

(fn `UserConstructionScript`
  (bind _containermesh (`self.ContainerMesh`))
  (if (`KismetSystemLibrary.IsServer`)
    (set `self.ThrowItemDirections` (`|MakeArray` (`self.ThrowItemDirection`) (`self.ThrowItemDirection1`)))
    (bind _returnvalue (`|GetDataTableRow` "/Game/Inventory/ContainerTypes_Table.ContainerTypes_Table" (`self.ContainerRowName`))
      (:`then`
        (bind (_containermesh_2 _meshscale _inventroysize) (break `/Game/Inventory/S_ContainerTypes` _returnvalue))
        (`StaticMeshComponent.SetStaticMesh` _containermesh _containermesh_2)
        (`SceneComponent.SetRelativeScale3D` _containermesh (`KismetMathLibrary.MakeVector` _meshscale _meshscale _meshscale))
        (set `self.InventorySize` _inventroysize)))))