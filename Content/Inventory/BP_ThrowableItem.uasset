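; BP_ThrowableItem is a thrown inventory item that turns into a pickup once it comes to rest.
; Server-side construction sets its mesh and scale from the TB_PickUpItemInfo row for ItemName.
; On BeginPlay the server enables physics and polls velocity through a Delay loop until the item nearly stops.
; It then spawns a pickup carrying ItemName and ItemContents, registers it with the game mode's BP_InvCompGamemode, and destroys itself.
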(event `self.ReceiveBeginPlay`
  (bind _returnvalue (`GameplayStatics.GetGameMode`))
  (bind _returnvalue_2 (`self.GetTransform`))
  (bind _itemmesh (`self.ItemMesh`))
  (if (`KismetSystemLibrary.IsServer`)
    (`PrimitiveComponent.SetSimulatePhysics` (`self.ItemMesh`) true)
    (`KismetSystemLibrary.Delay` 0.2 :!label _label)
    (if (>= (`KismetMathLibrary.VSize` (`self.GetVelocity`)) 5.0)
      (goto _label)
      (else
        (`PrimitiveComponent.SetSimulatePhysics` _itemmesh false)
        (`PrimitiveComponent.SetCollisionProfileName` _itemmesh "OverlapAllDynamic" true)
        (bind _returnvalue_3 (`|SpawnActorFromClass` "/Game/Inventory/BP_Pickup.BP_Pickup_C" (`KismetMathLibrary.MakeTransform` (.location _returnvalue_2) (`KismetMathLibrary.MakeRotator` 0.0 0.0 (.yaw (.rotation _returnvalue_2)))) "Undefined" "OverrideRootScale" null (`self.ItemName`) (`self.ItemContents`) null))
        (`/Engine/EditorBlueprintResources/StandardMacros.IsValid` _returnvalue_3
          (:`Is Valid`
            (cast `/Game/_CORE/Framework/BP_ThirdPersonGameMode` _returnvalue)
            (`/Game/Inventory/BP_InvCompGamemode.Add Saved Pickup Actor` (`self.GetComponentByClass` _returnvalue "/Game/Inventory/BP_InvCompGamemode.BP_InvCompGamemode_C") _returnvalue_3))
          (:`Is Not Valid`
            _))
        (`self.K2_DestroyActor`)))))

(fn `UserConstructionScript`
  (bind _itemmesh (`self.ItemMesh`))
  ;[0 0 0] ep 9 sets thrown item mesh
  (if (`KismetSystemLibrary.IsServer`)
    (bind _returnvalue (`|GetDataTableRow` "/Game/Inventory/TB_PickUpItemInfo.TB_PickUpItemInfo" (`self.ItemName`))
      (:`then`
        (bind (_pickupname _pickupmesh _pickupmesh_scale) (break `/Game/Inventory/S_PickUpItemInfo` _returnvalue))
        (`StaticMeshComponent.SetStaticMesh` _itemmesh _pickupmesh)
        (`SceneComponent.SetRelativeScale3D` _itemmesh (`KismetMathLibrary.MakeVector` _pickupmesh_scale _pickupmesh_scale _pickupmesh_scale))))))