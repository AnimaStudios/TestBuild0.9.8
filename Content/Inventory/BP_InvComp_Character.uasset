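; Character inventory component that manages a player's items and their interaction with pickups and containers.
; Svr_ events change the fixed-size slot array or pass container transfers to the GameMode component, while the Controller component handles UI and saving.
; Adding items applies data-table stack limits, splits overflow across slots and throws what won't fit as impulsed BP_ThrowableItem actors.
; Overlaps toggle item names and select the BPI_InteractableActor target for the interact input.
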(event `self.ReceiveBeginPlay`
  (bind _returnvalue (`self.GetOwner`))
  (if (`KismetSystemLibrary.IsServer`)
    (set `self.ThrowItemDirection` (`|GetArrayItem` (`Actor.GetComponentsByTag` _returnvalue "/Script/Engine.ArrowComponent" "InventoryComp")))
    (set `self.BP_InvComponent_Gamemode` (`Actor.GetComponentByClass` (`GameplayStatics.GetGameMode`) "/Game/Inventory/BP_InvCompGamemode.BP_InvCompGamemode_C"))
    (bind _ascharacter (cast `Character` _returnvalue))
    (bind _returnvalue_2 (`Pawn.GetController` _ascharacter))
    (`/Engine/EditorBlueprintResources/StandardMacros.IsValid` _returnvalue_2 :!label _label
      (:`Is Valid`
        (set `self.BP_InvComponent_Controller` (`Actor.GetComponentByClass` _returnvalue_2 "/Game/Inventory/BP_InvComp_Controller.BP_InvComp_Controller_C")))
      (:`Is Not Valid`
        (`KismetSystemLibrary.DelayUntilNextTick`)
        (goto _label)))))

(event `SaveCurrentInventory`
  (`/Game/Inventory/BP_InvComp_Controller.SaveInventoryToSaveGame` (`self.BP_InvComponent_Controller`) (`self.PlayerInventory`)))

(event `Svr_LoadInventoryFromSaveGame`
  (params (PlayerInventory :type "Array of /Game/Inventory/S_InventoryContents Structure"))
  (set `self.PlayerInventory` PlayerInventory)
  (bind _output_get (set `self.InventorySize` 21))
  (for _index (range (`KismetArrayLibrary.Array_Length` (`self.PlayerInventory`)) _output_get)
    (`KismetArrayLibrary.Array_Set` (`self.PlayerInventory`) _index (make `/Game/Inventory/S_InventoryContents` "Empty") true)))

(event `Svr_ClosedContainer`
  (bind _openedcontainer (`self.OpenedContainer`))
  (`/Engine/EditorBlueprintResources/StandardMacros.IsValid` _openedcontainer
    (:`Is Valid`
      (bind _returnvalue (`KismetArrayLibrary.Array_RemoveItem` (`/Game/Inventory/BP_Container.InteractingPlayers` _openedcontainer) self))
      (if _returnvalue
        (`KismetSystemLibrary.PrintString` "player removed from interactingplayers" true true (struct :`G` 1.0 :`B` 0.230514 :`A` 1.0))
        (else
          (`KismetSystemLibrary.PrintString` "player Not removed from interactingplayers" true true (struct :`R` 1.0 :`G` 0.065548 :`A` 1.0))))
      (set `self.OpenedContainer` null))))

(event `OpenContainer`
  (params (BP_Container :type "/Game/Inventory/BP_Container Object Reference"))
  (`/Game/Inventory/BP_InvComp_Controller.ContainerOpened` (`self.BP_InvComponent_Controller`) BP_Container))

(event `EnhancedInput|/Game/_CORE/Input/Actions/IA_OpenInventory`
  (params (ActionValue :type Boolean) (ElapsedSeconds :type "Float (double-precision)") (TriggeredSeconds :type "Float (double-precision)") (InputAction :type "InputAction Object Reference" :default "/Game/_CORE/Input/Actions/IA_OpenInventory.IA_OpenInventory"))
  (bind _bp_invcomponent_controller (`self.BP_InvComponent_Controller`))
  ;[0 0 0] Opens Inventory
  (:`Started`
    (`/Engine/EditorBlueprintResources/StandardMacros.IsValid` (`/Game/Inventory/BP_InvComp_Controller.WB_PlayerInventory` (`self.BP_InvComponent_Controller`))
      (:`Is Valid`
        (`Widget.RemoveFromParent` (`/Game/Inventory/BP_InvComp_Controller.WB_PlayerInventory` _bp_invcomponent_controller))
        (`/Game/Inventory/BP_InvComp_Controller.LeaveInventoryMenu` _bp_invcomponent_controller))
      (:`Is Not Valid`
        (`/Game/Inventory/BP_InvComp_Controller.UI_ShowInventoryMenu` _bp_invcomponent_controller)))))

(event `Svr_InteractWithInteractable`
  (bind _interactableactor (`self.InteractableActor`))
  (`/Engine/EditorBlueprintResources/StandardMacros.IsValid` _interactableactor
    (:`Is Valid`
      (`/Engine/EditorBlueprintResources/StandardMacros.IsValid` (`self.OpenedContainer`)
        (:`Is Not Valid`
          (message `/Game/Inventory/BPI_InteractableActor.InteractWithActor` _interactableactor self))))))

(event `EnhancedInput|/Game/_CORE/Input/Actions/IA_Interact`
  (params (ActionValue :type Boolean) (ElapsedSeconds :type "Float (double-precision)") (TriggeredSeconds :type "Float (double-precision)") (InputAction :type "InputAction Object Reference" :default "/Game/_CORE/Input/Actions/IA_Interact.IA_Interact"))
  (:`Started`
    (`self.Svr_InteractWithInteractable`)))

(event `LeaveContainerTrigger`
  (bind _bp_invcomponent_controller (`self.BP_InvComponent_Controller`))
  (`Widget.RemoveFromParent` (`/Game/Inventory/BP_InvComp_Controller.WB_PlayerInventory` _bp_invcomponent_controller))
  (`/Game/Inventory/BP_InvComp_Controller.LeaveInventoryMenu` _bp_invcomponent_controller))

(event `Svr_AddItemToContainer`
  (params (Contents :type "Array of /Game/Inventory/S_InventoryContents Structure (by ref)") (InventoryIndex :type Integer))
  (`/Game/Inventory/BP_InvCompGamemode.Add_ItemToContainer` (`self.BP_InvComponent_Gamemode`) Contents (`self.OpenedContainer`) InventoryIndex))

(event `Svr_RemoveItemFromContainer`
  (params (Contents :type "Array of /Game/Inventory/S_InventoryContents Structure (by ref)") (InventroyIndex :type Integer))
  (`/Game/Inventory/BP_InvCompGamemode.Remove_ItemFromContainer` (`self.BP_InvComponent_Gamemode`) Contents (`self.OpenedContainer`) InventroyIndex))

(event `Svr_AddItemToInventory`
  (params (PickupContents :type "Array of /Game/Inventory/S_InventoryContents Structure (by ref)") (BP_Pickup :type "/Game/Inventory/BP_Pickup Object Reference") (InventoryIndex :type Integer))
  (`self.AddItemToInvnetory` PickupContents BP_Pickup InventoryIndex))

(event `Svr_RemoveItemFromInventory`
  (params (ItemInfo :type "Array of /Game/Inventory/S_InventoryContents Structure (by ref)") (InventroyIndex :type Integer))
  (`self.RemoveItemFromInventory` ItemInfo InventroyIndex))

(event `Svr_TakeAllContainerItems`
  (bind _openedcontainer (`self.OpenedContainer`))
  (`self.AddItemToInvnetory` (`/Game/Inventory/BP_Container.ContainerContents` _openedcontainer) null -1)
  (`/Game/Inventory/BP_Container.ClearInventoryContents` _openedcontainer))

(event `Svr_ThrowItem`
  (params (ItemRowName :type Name) (Contents :type "Array of /Game/Inventory/S_InventoryContents Structure (by ref)") (IsFromContainer :type Boolean))
  (`self.ThrowItem` ItemRowName Contents IsFromContainer))

(event `BeginOverlap_Sphere`
  (params (Actor :type "Actor Object Reference"))
  (if (`KismetSystemLibrary.DoesImplementInterface` Actor "/Game/Inventory/BPI_InteractableActor.BPI_InteractableActor_C")
    (message `/Game/Inventory/BPI_InteractableActor.Set_ItemNameVisibility` Actor true)))

(event `EndOverlap_Sphere`
  (params (Actor :type "Actor Object Reference"))
  (if (`KismetSystemLibrary.DoesImplementInterface` Actor "/Game/Inventory/BPI_InteractableActor.BPI_InteractableActor_C")
    (message `/Game/Inventory/BPI_InteractableActor.Set_ItemNameVisibility` Actor false)))

(event `BeginOverlap_Mesh`
  (params (Actor :type "Actor Object Reference"))
  (if (`KismetSystemLibrary.DoesImplementInterface` Actor "/Game/Inventory/BPI_InteractableActor.BPI_InteractableActor_C")
    (set `self.InteractableActor` Actor)
    (bind _hinttext (message `/Game/Inventory/BPI_InteractableActor.Get_InteractHintText` Actor))
    (`/Game/Inventory/BP_InvComp_Controller.Hud_SetInteractHint` (`self.BP_InvComponent_Controller`) true _hinttext)))

(event `EndOverlap_Mesh`
  (params (Actor :type "Actor Object Reference"))
  (if (== Actor (`self.InteractableActor`))
    (set `self.InteractableActor` null)
    (`/Engine/EditorBlueprintResources/StandardMacros.IsValid` (`self.OpenedContainer`)
      (:`Is Valid`
        (`self.LeaveContainerTrigger`))
      (:`Is Not Valid`
        _))
    (`/Game/Inventory/BP_InvComp_Controller.Hud_SetInteractHint` (`self.BP_InvComponent_Controller`) false "")))

(fn `AddItemToInvnetory`
  (params (PickupContents :type "Array of /Game/Inventory/S_InventoryContents Structure") (BP_Pickup :type "/Game/Inventory/BP_Pickup Object Reference") (InventoryIndex :type Integer))
  (locals (Lol_InventoryIndex :type Integer) (Lol_Plr_InventoryContents :type "/Game/Inventory/S_InventoryContents Structure") (Lol_InventroyToAdd :type "/Game/Inventory/S_InventoryContents Structure") (Lol_IsSlotFound :type Boolean) (Lcl_CanStackItem :type Boolean) (Lcl_IsStackLimited :type Boolean) (Lcl_MaxStackSize :type Integer) (Lcl_AllItemsAdded :type Boolean) (Lcl_NewStackSize :type Integer) (Lcl_AmountLeftToAdd :type Integer))
  (bind (_itemrowname _itemamount) (break `/Game/Inventory/S_InventoryContents` (`local.Lol_InventroyToAdd`)))
  (bind (_itemrowname_2 _itemamount_2) (break `/Game/Inventory/S_InventoryContents` (`local.Lol_InventroyToAdd`)))
  (bind (_itemrowname_3 _itemamount_3) (break `/Game/Inventory/S_InventoryContents` (`local.Lol_Plr_InventoryContents`)))
  (for _array_element PickupContents
    (if (!= (`.ItemRowNAme_3_03A6F83347ECA63487A0DAA65D30ACFB` (break `/Game/Inventory/S_InventoryContents` _array_element)) "Empty")
      (bind _output_get (set `local.Lol_InventroyToAdd` _array_element))
      (bind _output_get_2 (set `local.Lol_InventoryIndex` InventoryIndex))
      (set `local.Lol_Plr_InventoryContents` (`|GetArrayItem` (`self.PlayerInventory`) _output_get_2))
      (bind _returnvalue (`|GetDataTableRow` "/Game/Inventory/TB_PickUpItemInfo.TB_PickUpItemInfo" (`.ItemRowNAme_3_03A6F83347ECA63487A0DAA65D30ACFB` (break `/Game/Inventory/S_InventoryContents` _output_get)))
        (:`then`
          (bind (_pickupname _pickupmesh _pickupmesh_scale _showpickupname _pickupmeshoffset _hud_icon _maxstacksize) (break `/Game/Inventory/S_PickUpItemInfo` _returnvalue))
          (switch `int` _maxstacksize
            (:`Default`
              (set `local.Lcl_CanStackItem` true)
              (set `local.Lcl_IsStackLimited` true)
              (set `local.Lcl_MaxStackSize` _maxstacksize))
            (:`-1`
              (set `local.Lcl_CanStackItem` false)
              (set `local.Lcl_IsStackLimited` true)
              (set `local.Lcl_MaxStackSize` 1))
            (:`0`
              (set `local.Lcl_CanStackItem` true)
              (set `local.Lcl_IsStackLimited` false)))
          (set `local.Lcl_AllItemsAdded` true :!label _label)
          (set `local.Lcl_NewStackSize` 0)
          (set `local.Lcl_AmountLeftToAdd` 0)
          (set `local.Lol_IsSlotFound` false)
          (if (< (`local.Lol_InventoryIndex`) 0)
            (for (_array_element_2 _array_index) (`self.PlayerInventory`) :!label _label_2
              (if (== (`.ItemRowNAme_3_03A6F83347ECA63487A0DAA65D30ACFB` (break `/Game/Inventory/S_InventoryContents` _array_element_2)) "Empty")
                (set `local.Lol_IsSlotFound` true)
                (set `local.Lol_InventoryIndex` _array_index)
                (break)))
            (if (`local.Lol_IsSlotFound`)
              (set `local.Lcl_NewStackSize` (`.ItemAmount_6_5F407C944CCD8EFBF9780CB5F8F7A858` (break `/Game/Inventory/S_InventoryContents` (`local.Lol_InventroyToAdd`))) :!label _label_3)
              (if (`local.Lcl_IsStackLimited`)
                (if (not (<= (`local.Lcl_NewStackSize`) (`local.Lcl_MaxStackSize`)))
                  (set `local.Lcl_AmountLeftToAdd` (- (`local.Lcl_NewStackSize`) (`local.Lcl_MaxStackSize`)))
                  (set `local.Lcl_NewStackSize` (`local.Lcl_MaxStackSize`))
                  (set `local.Lcl_AllItemsAdded` false)))
              (`KismetArrayLibrary.Array_Set` (`self.PlayerInventory`) (`local.Lol_InventoryIndex`) (make `/Game/Inventory/S_InventoryContents` (`.ItemRowNAme_3_03A6F83347ECA63487A0DAA65D30ACFB` (break `/Game/Inventory/S_InventoryContents` (`local.Lol_InventroyToAdd`))) (`local.Lcl_NewStackSize`)) true)
              (if (`local.Lcl_AllItemsAdded`) :!label _label_4
                _
                (else
                  (setmembers `/Game/Inventory/S_InventoryContents` :`StructRef` (`local.Lol_InventroyToAdd`) :`ItemAmount` (`local.Lcl_AmountLeftToAdd`))
                  (set `local.Lol_InventoryIndex` -1)
                  (goto _label)))
              (else
                (if (`local.Lcl_CanStackItem`)
                  (for (_array_element_3 _array_index_2) (`self.PlayerInventory`)
                    (bind (_itemrowname_4 _itemamount_4) (break `/Game/Inventory/S_InventoryContents` _array_element_3))
                    (if (== _itemrowname_4 (`.ItemRowNAme_3_03A6F83347ECA63487A0DAA65D30ACFB` (break `/Game/Inventory/S_InventoryContents` (`local.Lol_InventroyToAdd`))))
                      (if (or (and (`local.Lcl_CanStackItem`) (not (`local.Lcl_IsStackLimited`))) (and (`local.Lcl_CanStackItem`) (`local.Lcl_IsStackLimited`) (< _itemamount_4 (`local.Lcl_MaxStackSize`))))
                        (set `local.Lol_IsSlotFound` true)
                        (set `local.Lol_InventoryIndex` _array_index_2)
                        (set `local.Lol_Plr_InventoryContents` _array_element_3)
                        (break))))
                  (if (`local.Lol_IsSlotFound`)
                    (set `local.Lcl_NewStackSize` (+ _itemamount_3 (`.ItemAmount_6_5F407C944CCD8EFBF9780CB5F8F7A858` (break `/Game/Inventory/S_InventoryContents` (`local.Lol_InventroyToAdd`)))) :!label _label_5)
                    (if (`local.Lcl_IsStackLimited`)
                      (if (not (<= (`local.Lcl_NewStackSize`) (`local.Lcl_MaxStackSize`)))
                        (set `local.Lcl_AmountLeftToAdd` (- (`local.Lcl_NewStackSize`) (`local.Lcl_MaxStackSize`)))
                        (set `local.Lcl_NewStackSize` (`local.Lcl_MaxStackSize`))
                        (set `local.Lcl_AllItemsAdded` false)))
                    (`KismetArrayLibrary.Array_Set` (`self.PlayerInventory`) (`local.Lol_InventoryIndex`) (make `/Game/Inventory/S_InventoryContents` _itemrowname_3 (`local.Lcl_NewStackSize`)) true)
                    (goto _label_4)
                    (else
                      (`KismetSystemLibrary.PrintString` "inventroy full cannot add item" true true (struct :`R` 1.0 :`B` 0.083431 :`A` 1.0) 15.0)))
                  (else
                    (`KismetSystemLibrary.PrintString` "Inventory full! Item cannot stack!" true true (struct :`R` 1.0 :`G` 0.203125 :`B` 0.221132 :`A` 1.0) 5.0)))
                (`self.ThrowItem` _itemrowname_2 (`|MakeArray` (make `/Game/Inventory/S_InventoryContents` _itemrowname_2 _itemamount_2)))))
            (elif (== (`.ItemRowNAme_3_03A6F83347ECA63487A0DAA65D30ACFB` (break `/Game/Inventory/S_InventoryContents` (`local.Lol_Plr_InventoryContents`))) (`.ItemRowNAme_3_03A6F83347ECA63487A0DAA65D30ACFB` (break `/Game/Inventory/S_InventoryContents` (`local.Lol_InventroyToAdd`))))
              (if (`local.Lcl_CanStackItem`)
                (goto _label_5)
                (else
                  (goto _label_2)))
              (elif (== (`.ItemRowNAme_3_03A6F83347ECA63487A0DAA65D30ACFB` (break `/Game/Inventory/S_InventoryContents` (`local.Lol_Plr_InventoryContents`))) "Empty")
                (goto _label_3)
                (else
                  (goto _label_2)))))
          (`/Game/Inventory/BP_InvComp_Controller.ClientHud_UpdateNewsFeed` (`self.BP_InvComponent_Controller`) _itemrowname _itemamount true)))))
  (`/Engine/EditorBlueprintResources/StandardMacros.IsValid` (`local.BP_Pickup`)
    (:`Is Valid`
      (`/Game/Inventory/BP_InvCompGamemode.Remove_SavedPickupActor` (`self.BP_InvComponent_Gamemode`) null))
    (:`Is Not Valid`
      _))
  (`self.SaveCurrentInventory`)
  (`/Game/Inventory/BP_InvComp_Controller.HUD_UpdateInventoryGrid` (`self.BP_InvComponent_Controller`) (`self.PlayerInventory`) true false)
  (return))

(fn `RemoveItemFromInventory`
  (params (ItemInfo :type "Array of /Game/Inventory/S_InventoryContents Structure") (InventroyIndex :type Integer))
  (locals (Lcl_NewAmount :type Integer))
  (bind (_itemrowname _itemamount) (break `/Game/Inventory/S_InventoryContents` (`|GetArrayItem` (`local.ItemInfo`))))
  (bind (_itemrowname_2 _itemamount_2) (break `/Game/Inventory/S_InventoryContents` (`|GetArrayItem` (`self.PlayerInventory`) InventroyIndex)))
  (if (`KismetArrayLibrary.Array_IsNotEmpty` (`self.PlayerInventory`))
    (bind _output_get (set `local.Lcl_NewAmount` (- _itemamount_2 (`.ItemAmount_6_5F407C944CCD8EFBF9780CB5F8F7A858` (break `/Game/Inventory/S_InventoryContents` (`|GetArrayItem` ItemInfo))))))
    (if (<= _output_get 0)
      (`KismetArrayLibrary.Array_Set` (`self.PlayerInventory`) InventroyIndex (make `/Game/Inventory/S_InventoryContents` "Empty") true)
      (else
        (`KismetArrayLibrary.Array_Set` (`self.PlayerInventory`) InventroyIndex (make `/Game/Inventory/S_InventoryContents` _itemrowname_2 (`local.Lcl_NewAmount`)) true)))
    (`self.SaveCurrentInventory`)
    (`/Game/Inventory/BP_InvComp_Controller.HUD_UpdateInventoryGrid` (`self.BP_InvComponent_Controller`) (`self.PlayerInventory`) true false)
    (`/Game/Inventory/BP_InvComp_Controller.ClientHud_UpdateNewsFeed` (`self.BP_InvComponent_Controller`) _itemrowname _itemamount false)
    (return)))

(fn `ThrowItem`
  (params (ItemRowName :type Name) (Contents :type "Array of /Game/Inventory/S_InventoryContents Structure") (IsFromContainer :type Boolean))
  (locals (Lol_throwDirection :type "ArrowComponent Object Reference"))
  (bind _throwitemdirection (`self.ThrowItemDirection`))
  (if IsFromContainer
    (bind _output_get (set `local.Lol_throwDirection` (`KismetArrayLibrary.Array_Random` (`/Game/Inventory/BP_Container.ThrowItemDirections` (`self.OpenedContainer`)))))
    (bind _returnvalue (`|SpawnActorFromClass` "/Game/Inventory/BP_ThrowableItem.BP_ThrowableItem_C" (`SceneComponent.K2_GetComponentToWorld` _output_get) "Undefined" "OverrideRootScale" null ItemRowName Contents null))
    (`PrimitiveComponent.AddImpulse` (`/Game/Inventory/BP_ThrowableItem.ItemMesh` _returnvalue) (* (`SceneComponent.GetForwardVector` (`local.Lol_throwDirection`)) 250) "None" true)
    (else
      (bind _returnvalue_2 (`|SpawnActorFromClass` "/Game/Inventory/BP_ThrowableItem.BP_ThrowableItem_C" (`SceneComponent.K2_GetComponentToWorld` _throwitemdirection) "Undefined" "OverrideRootScale" null ItemRowName Contents null))
      (`PrimitiveComponent.AddImpulse` (`/Game/Inventory/BP_ThrowableItem.ItemMesh` _returnvalue_2) (* (`SceneComponent.GetForwardVector` _throwitemdirection) 250) "None" true))))