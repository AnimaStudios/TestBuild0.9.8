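; Base spell actor with projectile movement that configures itself from the DT_Spells data table.
; The Construction Script converts the SpellInfo spell name enum to a row name and, if found, overwrites SpellInfo with that row.
; The row's speed and gravity scale then drive ProjectileMovement, with initial and max speed set equal.
; The event graph holds no active logic.
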(fn `UserConstructionScript`
  (bind _projectilemovement (`self.ProjectileMovement`))
  (bind _returnvalue (`|GetDataTableRow` "/Game/_CORE/Magic/DT_Spells.DT_Spells" (`KismetStringLibrary.Conv_StringToName` (`|GetEnumeratorNameAsString` (`.SpellName_9_B78667114FDB009C3CD7718C75BC94ED` (break `/Game/_CORE/Magic/S_Spell_Info` (`self.SpellInfo`))))))
    (:`then`
      (bind _output_get (set `self.SpellInfo` _returnvalue))
      (bind (_spellclass _spellname _spelltype _spellimage _manacost _potency _price _speed _gravityscale) (break `/Game/_CORE/Magic/S_Spell_Info` _output_get))
      (set `ProjectileMovementComponent.InitialSpeed` _speed _projectilemovement)
      (set `ProjectileMovementComponent.MaxSpeed` _speed _projectilemovement)
      (set `ProjectileMovementComponent.ProjectileGravityScale` _gravityscale _projectilemovement))))