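; Equipment component for the player character that handles weapon pickup, inventory storage and the equipment menu.
; Interact sphere-traces forward from the third-person camera, adds a hit BP_Weapon's item data to WeaponSlots and destroys the actor.
; The menu input toggles the WB_Equipment widget, switching input mode, cursor visibility and character movement.
; A debug key prints the stored items' row names.
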(event Input|EnhancedActionEvents|EnhancedInputActionIA_Interact
  (params (ActionValue :type Boolean) (ElapsedSeconds :type Float%20%28double-precision%29) (TriggeredSeconds :type Float%20%28double-precision%29) (InputAction :type Input%20Action%20Object%20Reference :default "/Game/_CORE/Input/Actions/IA_Interact.IA_Interact"))
  (bind _tpp_follow_camera (Variables|Default|GetTPP%20Follow%20Camera))
  (bind _returnvalue (Transformation|GetWorldLocation _tpp_follow_camera))
  ;[0 0 0] Pick Up Trace
  (:Started
    (bind (_outhit _returnvalue_2) (Collision|SphereTraceForObjects _returnvalue (+ _returnvalue (* (Math|Vector|GetForwardVector (Transformation|GetWorldRotation _tpp_follow_camera)) 1e+03)) 15.0 (Utilities|Array|MakeArray "ObjectTypeQuery2") false 0 "ForDuration"))
    (if _returnvalue_2
      (bind _asbp_weapon (Utilities|Casting|CastToBP_Weapon (.HitActor (Collision|BreakHitResult _outhit))))
      (CallFunction|AddWeapon (Variables|/Game/_CORE/EquipmentSystem/BP_Weapon.BP_Weapon_C|GetItemData _asbp_weapon))
      (Actor|DestroyActor _asbp_weapon)
      (Development|PrintString "Item Pickedup"))))

(event Input|EnhancedActionEvents|EnhancedInputActionIA_EquipmentMenu
  (params (ActionValue :type Boolean) (ElapsedSeconds :type Float%20%28double-precision%29) (TriggeredSeconds :type Float%20%28double-precision%29) (InputAction :type Input%20Action%20Object%20Reference :default "/Game/_CORE/Input/Actions/IA_EquipmentMenu.IA_EquipmentMenu"))
  (bind _returnvalue (Game|GetPlayerController 0))
  ;[0 0 0] Equipment menu
  (:Started
    (if (not (Variables|Default|GetIsPanelOpened))
      (Variables|Default|SetIsPanelOpened true)
      (bind _returnvalue_2 (UserInterface|CreateWidget "/Game/_CORE/Widjets/WB_Equipment.WB_Equipment_C"))
      (bind _output_get (Variables|Default|SetEquipmentWidjet _returnvalue_2))
      (UserInterface|Viewport|AddtoViewport _output_get 0)
      (Input|SetInputModeGameandUI _returnvalue (Variables|Default|GetEquipmentWidjet) "DoNotLock" true false)
      (Variables|/Script/Engine.PlayerController|SetbShowMouseCursor _returnvalue true)
      (bind _asbp_devol_base_character (Utilities|Casting|CastToBP_Devol_BaseCharacter (Components|GetOwner)))
      (Pawn|Components|CharacterMovement|SetMovementMode (Variables|/Script/Engine.Character|GetCharacterMovement _asbp_devol_base_character) "MOVE_None" 0)
      (else
        (Variables|Default|SetIsPanelOpened false)
        (bind _equipmentwidjet (Variables|Default|GetEquipmentWidjet)
          (:then
            (Widget|RemovefromParent _equipmentwidjet)
            (Variables|Default|SetEquipmentWidjet 0)
            (Input|SetInputModeGameOnly _returnvalue false)
            (Variables|/Script/Engine.PlayerController|SetbShowMouseCursor _returnvalue false)
            (bind _asbp_devol_base_character_2 (Utilities|Casting|CastToBP_Devol_BaseCharacter (Components|GetOwner)))
            (Pawn|Components|CharacterMovement|SetMovementMode (Variables|/Script/Engine.Character|GetCharacterMovement _asbp_devol_base_character_2) "MOVE_Walking" 0))
          (:else))))))

(event EventBeginPlay
  (bind _asbp_devol_base_character (Utilities|Casting|CastToBP_Devol_BaseCharacter (Components|GetOwner)))
  (Variables|Default|SetTPP%20Follow%20Camera (Variables|/Game/_CORE/Charcaters/BP_Devol_BaseCharacter.BP_Devol_BaseCharacter_C|GetTPP_FollowCamera _asbp_devol_base_character)))

(event Input|KeyboardEvents|DebugKeyH
  (params (Key :type Key%20Structure :default "None") (ActionValue :type Input%20Action%20Value%20Structure))
  ;[0 0 0] Show inventory
  (:Pressed
    (for _array_element (Variables|Default|GetWeaponSlots)
      (Development|PrintString (Utilities|String|ToString(Name) (.RowName (Utilities|Struct|BreakDataTableRowHandle (Utilities|Struct|BreakS_Slots _array_element)))) true true "(R=0.000000,G=0.660000,B=1.000000,A=1.000000)" 5.0))))

(fn AddWeapon
  (params (NewItem :type S%20Slots%20Structure%20%28by%20ref%29))
  (Utilities|Array|Add (Variables|Default|GetWeaponSlots) NewItem))