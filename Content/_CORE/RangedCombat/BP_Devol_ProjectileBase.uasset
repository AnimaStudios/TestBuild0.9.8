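; Base projectile actor for ranged combat that flies with configurable speed and gravity, applied to its projectile movement in the construction script.
; Its collision box ignores the instigator, or the owner as fallback, so shooters do not hit themselves.
; On hit it broadcasts the impact with actor and hit data, spawns effect and sound at that location, then destroys itself.
; Projectiles that hit nothing expire after a fixed delay.
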(event `self.ReceiveBeginPlay`
  (bind _returnvalue (`self.GetInstigator`))
  ;[0 0 0] Ignores the Caster so they dont shoot themselves
  (`PrimitiveComponent.IgnoreActorWhenMoving` (`self.BoxCollision`) (select `bool` (`KismetSystemLibrary.IsValid` _returnvalue) :`false` (`self.GetOwner`) :`true` _returnvalue :!type "Actor Object Reference") true)
  (`KismetSystemLibrary.Delay` 15.0)
  (`self.K2_DestroyActor`))

(event `self.BoxCollision.OnComponentHit`
  (params (HitComponent :type "PrimitiveComponent Object Reference") (OtherActor :type "Actor Object Reference") (OtherComp :type "PrimitiveComponent Object Reference") (NormalImpulse :type "Vector Structure") (Hit :type "HitResult Structure (by ref)"))
  (bind (_bblockinghit _binitialoverlap _time _distance _location) (`GameplayStatics.BreakHitResult` Hit))
  ;[0 0 0] On Impact destroys itself, plays sound/effects
  (`self.OnProjectileImpact` OtherActor Hit)
  (`NiagaraFunctionLibrary.SpawnSystemAtLocation` (`self.ImpactEffect`) _location)
  (`GameplayStatics.PlaySoundAtLocation` (`self.ImpactSound`) _location (struct) 1.0 1.0 0.0 null null null null)
  (`self.K2_DestroyActor`))

(fn `UserConstructionScript`
  (bind _projectilemovement (`self.ProjectileMovement`))
  (set `ProjectileMovementComponent.InitialSpeed` (`self.Speed`) _projectilemovement)
  (set `ProjectileMovementComponent.MaxSpeed` (`self.Speed`) _projectilemovement)
  (set `ProjectileMovementComponent.ProjectileGravityScale` (`self.Gavity`) _projectilemovement))